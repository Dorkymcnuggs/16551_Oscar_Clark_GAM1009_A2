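; Player controller for the shoot-em-up that owns the player pawn's HUD widget.
; On BeginPlay it creates and displays the widget, and on possessing a pawn it sends that pawn a health value of 100.
; EndPlay removes and clears the widget, then forces garbage collection to avoid health-widget errors after respawn.
; The ApplyStatPickUp function is an empty stub.
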(event `self.ReceiveEndPlay`
  (params (EndPlayReason :type "EEndPlayReason Enum" :default "Destroyed"))
  ;[0.07835 0.2413 0.07835] Helps avoid error when loading health widget after player respawn
  (`Widget.RemoveFromParent` (`self.ControlHUDRef`))
  (set `self.ControlHUDRef` null)
  (`KismetSystemLibrary.CollectGarbage`))

(event `self.ReceiveBeginPlay`
  ;[0.07835 0.2413 0.07835] Helps avoid error when loading health widget after player respawn
  (bind _returnvalue (`|CreateWidget` "/Game/Widgets/WBP_PlayerPawnWidget.WBP_PlayerPawnWidget_C"))
  (bind _output_get (set `self.ControlHUDRef` _returnvalue))
  (`UserWidget.AddToViewport` _output_get 0))

(event `self.ReceivePossess`
  (params (PossessedPawn :type "Pawn Object Reference"))
  ;[0.07835 0.2413 0.07835] Helps avoid error when loading health widget after player respawn
  (message `/Game/GameFrame/BPI_SCHMUP.SetHealth` PossessedPawn 100.0))

(fn `ApplyStatPickUp`
  (returns (Stats :type "/Game/GameFrame/S_Pickup Structure"))
  (return))

(fn `UserConstructionScript`)