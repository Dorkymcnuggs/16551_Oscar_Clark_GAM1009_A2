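; BP_Enemy_Spawner is an actor that continuously spawns enemies along a line between two limit components.
; On BeginPlay it starts a looping timer that fires SpawnEnemy every three seconds.
; Each spawn randomly picks BP_Enemy_A or BP_Enemy_B, places it at a random lerp between LeftSpawnLim and RightSpawnLim, and takes the left limit's rotation.
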(event `self.ReceiveBeginPlay`
  (`KismetSystemLibrary.K2_SetTimerDelegate` (delegate `SpawnEnemy`) 3.0 true))

(event `SpawnEnemy`
  (`|SpawnActorFromClass` (`|GetArrayItem` (`|MakeArray` "/Game/Blueprints/BP_Enemy_A.BP_Enemy_A_C" "/Game/Blueprints/BP_Enemy_B.BP_Enemy_B_C" :!type "Actor Class Reference") (`KismetMathLibrary.RandomInteger` 2)) (`KismetMathLibrary.MakeTransform` (`KismetMathLibrary.VLerp` (`SceneComponent.K2_GetComponentLocation` (`self.LeftSpawnLim`)) (`SceneComponent.K2_GetComponentLocation` (`self.RightSpawnLim`)) (`KismetMathLibrary.RandomFloat`)) (`SceneComponent.K2_GetComponentRotation` (`self.LeftSpawnLim`))) "Undefined" "MultiplyWithRoot" null null))

(fn `UserConstructionScript`)