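; Player-controlled tank Blueprint that drives with W/S, turns with A/D and rotates its TankTop component with Q/E.
; Each key opens a Gate on press and closes it on release, while a Tick Sequence feeds all six gates.
; Open gates apply delta-time-scaled local offsets or rotations, with sweep on movement.
; Space Bar only prints "Bang!" as a firing stand-in.
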(event `self.ReceiveBeginPlay`)

(event `Key|SpaceBar`
  (params (Key :type "Key Structure"))
  (:`Pressed`
    (`KismetSystemLibrary.PrintString` "Bang!")))

(event `Key|W`
  (params (Key :type "Key Structure"))
  (:`Pressed`
    (goto _label :!via `Open`))
  (:`Released`
    (goto _label :!via `Close`)))

(event `self.ReceiveTick`
  (params (DeltaSeconds :type "Float (single-precision)"))
  (`|ExecutionSequence`
    (:`then_0`
      (`/Engine/EditorBlueprintResources/StandardMacros.Gate` true :!label _label
        (:`Exit`
          (`self.K2_AddActorLocalOffset` (* (100.0 0.0 0.0) (`GameplayStatics.GetWorldDeltaSeconds`)) true))))
    (:`then_1`
      (`/Engine/EditorBlueprintResources/StandardMacros.Gate` true :!label _label_2
        (:`Exit`
          (`self.K2_AddActorLocalOffset` (* (-100.0 0.0 0.0) (`GameplayStatics.GetWorldDeltaSeconds`)) true))))
    (:`then_2`
      (`/Engine/EditorBlueprintResources/StandardMacros.Gate` true :!label _label_3
        (:`Exit`
          (`self.K2_AddActorLocalRotation` (* (struct :`Yaw` -30.0) (`GameplayStatics.GetWorldDeltaSeconds`))))))
    (:`then_3`
      (`/Engine/EditorBlueprintResources/StandardMacros.Gate` true :!label _label_4
        (:`Exit`
          (`self.K2_AddActorLocalRotation` (* (struct :`Yaw` 30.0) (`GameplayStatics.GetWorldDeltaSeconds`))))))
    (:`then_4`
      (`/Engine/EditorBlueprintResources/StandardMacros.Gate` true :!label _label_5
        (:`Exit`
          (`SceneComponent.K2_AddLocalRotation` (`self.TankTop`) (* (struct :`Yaw` -20.0) (`GameplayStatics.GetWorldDeltaSeconds`)) false false))))
    (:`then_5`
      (`/Engine/EditorBlueprintResources/StandardMacros.Gate` true :!label _label_6
        (:`Exit`
          (`SceneComponent.K2_AddLocalRotation` (`self.TankTop`) (* (struct :`Yaw` 20.0) (`GameplayStatics.GetWorldDeltaSeconds`)) false false))))))

(event `Key|S`
  (params (Key :type "Key Structure"))
  (:`Pressed`
    (goto _label_2 :!via `Open`))
  (:`Released`
    (goto _label_2 :!via `Close`)))

(event `Key|A`
  (params (Key :type "Key Structure"))
  (:`Pressed`
    (goto _label_3 :!via `Open`))
  (:`Released`
    (goto _label_3 :!via `Close`)))

(event `Key|D`
  (params (Key :type "Key Structure"))
  (:`Pressed`
    (goto _label_4 :!via `Open`))
  (:`Released`
    (goto _label_4 :!via `Close`)))

(event `Key|Q`
  (params (Key :type "Key Structure"))
  (:`Pressed`
    (goto _label_5 :!via `Open`))
  (:`Released`
    (goto _label_5 :!via `Close`)))

(event `Key|E`
  (params (Key :type "Key Structure"))
  (:`Pressed`
    (goto _label_6 :!via `Open`))
  (:`Released`
    (goto _label_6 :!via `Close`)))

(fn `UserConstructionScript`)