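; Player-controlled helicopter pawn for a shoot-'em-up, which adds the SHMUP input mapping context when possessed.
; Enhanced Input actions drive FloatingPawnMovement along the Arrow's forward and right vectors and the world Z axis.
; The fire action spawns a player bullet at the Arrow's transform after a short delay.
; Tick smooths actor rotation by interpolating pitch and roll from movement input and yaw toward the Arrow's heading.
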(event `self.ReceivePossessed`
  (params (NewController :type "Controller Object Reference"))
  ; Basic movement and shooting
  (bind _asplayer_controller (cast `PlayerController` NewController))
  (`EnhancedInputSubsystemInterface.AddMappingContext` (pcsubsystem `EnhancedInputLocalPlayerSubsystem` _asplayer_controller) "/Game/Inputs/IMC_SHMUP.IMC_SHMUP" 0 (struct)))

(event `EnhancedInput|/Game/Inputs/IA_MoveFowBack`
  (params (ActionValue :type "Float (double-precision)") (ElapsedSeconds :type "Float (double-precision)") (TriggeredSeconds :type "Float (double-precision)") (InputAction :type "InputAction Object Reference" :default "/Game/Inputs/IA_MoveFowBack.IA_MoveFowBack"))
  (bind (_returnvalue_x _returnvalue_y) (`KismetMathLibrary.BreakVector` (* ActionValue (`SceneComponent.GetForwardVector` (`self.Arrow`)))))
  ; Basic movement and shooting
  (:`Triggered`
    (`PawnMovementComponent.AddInputVector` (`self.FloatingPawnMovement`) (`KismetMathLibrary.MakeVector` _returnvalue_x _returnvalue_y) false)))

(event `EnhancedInput|/Game/Inputs/IA_MoveLeftRight`
  (params (ActionValue :type "Float (double-precision)") (ElapsedSeconds :type "Float (double-precision)") (TriggeredSeconds :type "Float (double-precision)") (InputAction :type "InputAction Object Reference" :default "/Game/Inputs/IA_MoveLeftRight.IA_MoveLeftRight"))
  (bind (_returnvalue_x _returnvalue_y) (`KismetMathLibrary.BreakVector` (* ActionValue (`SceneComponent.GetRightVector` (`self.Arrow`)))))
  ; Basic movement and shooting
  (:`Triggered`
    (`PawnMovementComponent.AddInputVector` (`self.FloatingPawnMovement`) (`KismetMathLibrary.MakeVector` _returnvalue_x _returnvalue_y) false)))

(event `EnhancedInput|/Game/Inputs/IA_MoveUpDown`
  (params (ActionValue :type "Float (double-precision)") (ElapsedSeconds :type "Float (double-precision)") (TriggeredSeconds :type "Float (double-precision)") (InputAction :type "InputAction Object Reference" :default "/Game/Inputs/IA_MoveUpDown.IA_MoveUpDown"))
  ; Basic movement and shooting
  (:`Triggered`
    (`PawnMovementComponent.AddInputVector` (`self.FloatingPawnMovement`) (`KismetMathLibrary.MakeVector` 0.0 0.0 ActionValue) false)))

(event `EnhancedInput|/Game/Inputs/IA_1stFire`
  (params (ActionValue :type Boolean) (ElapsedSeconds :type "Float (double-precision)") (TriggeredSeconds :type "Float (double-precision)") (InputAction :type "InputAction Object Reference" :default "/Game/Inputs/IA_1stFire.IA_1stFire"))
  (bind (_returnvalue_location _returnvalue_rotation) (`KismetMathLibrary.BreakTransform` (`SceneComponent.K2_GetComponentToWorld` (`self.Arrow`))))
  ; Basic movement and shooting
  (:`Triggered`
    (`KismetSystemLibrary.Delay` 0.1)
    (`|SpawnActorFromClass` "/Game/Blueprints/BP_ProjectileBase_PlayerBullet.BP_ProjectileBase_PlayerBullet_C" (`KismetMathLibrary.MakeTransform` _returnvalue_location _returnvalue_rotation) "AdjustIfPossibleButDontSpawnIfColliding" "MultiplyWithRoot" null null)))

(event `self.ReceiveTick`
  (params (DeltaSeconds :type "Float (single-precision)"))
  (bind (_returnvalue_roll _returnvalue_pitch _returnvalue_yaw) (`KismetMathLibrary.BreakRotator` (`SceneComponent.K2_GetComponentRotation` (`self.Arrow`))))
  ; Handles Smoooth movement (interpoling)
  (`|ExecutionSequence`
    (:`then_0`
      (bind _output_get (set `self.TargetPitch` (* (`|GetInputActionValue`) -1.0)))
      (bind _output_get_2 (set `self.CurrentPitch` (`KismetMathLibrary.FInterpTo` (`self.CurrentPitch`) _output_get (`GameplayStatics.GetWorldDeltaSeconds`) 1.0))))
    (:`then_1`
      (bind _output_get_3 (set `self.TargetRoll` (* (`|GetInputActionValue`) -1.0)))
      (bind _output_get_4 (set `self.CurrentRoll` (`KismetMathLibrary.FInterpTo` (`self.CurrentRoll`) _output_get_3 (`GameplayStatics.GetWorldDeltaSeconds`) 1.0))))
    (:`then_2`
      (bind _output_get_5 (set `self.TargetYAW` _returnvalue_yaw))
      (bind (_returnvalue_roll_2 _returnvalue_pitch_2 _returnvalue_yaw_2) (`KismetMathLibrary.BreakRotator` (`KismetMathLibrary.RInterpTo` (`KismetMathLibrary.MakeRotator` 0.0 0.0 (`self.CurrentYAW`)) (`KismetMathLibrary.MakeRotator` 0.0 0.0 _output_get_5) (`GameplayStatics.GetWorldDeltaSeconds`))))
      (bind _output_get_6 (set `self.CurrentYAW` _returnvalue_yaw_2))))
  (`self.K2_SetActorRotation` (`KismetMathLibrary.MakeRotator` (* _output_get_4 (`self.MaxRoll`)) (* _output_get_2 (`self.MaxPitch`)) _output_get_6)))

(fn `UserConstructionScript`)