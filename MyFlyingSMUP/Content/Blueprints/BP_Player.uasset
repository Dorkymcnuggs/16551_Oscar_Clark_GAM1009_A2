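; Player plane pawn for a shoot-'em-up, with Enhanced Input movement, cursor aiming, health and a pause screen.
; Tick turns RotationalOffset toward the cursor hit and interpolates actor pitch and roll from move input and yaw from the Arrow, which also orients movement and shots.
; Delayed bullet and missile fire each have two patterns, toggled by a Left Alt debug key.
; Damage updates the HUD widget, then flashes an overlay or respawns at zero health.
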(event Custom|Hit%20Sequence
  ;[0.15 0.15 0.15 0.5] Player receive damage as hit
  (Audio|PlaySound2D "/Game/AudioFile/MS_Hit.MS_Hit" 1.0 1.0 0.0 0 0)
  (Rendering|Material|SetOverlayMaterial (Variables|Default|GetSM_Plane_Body) "/Game/Materials/M_OverlayDamage.M_OverlayDamage" :!class /Script/Engine.MeshComponent)
  (Utilities|FlowControl|Delay 2.0)
  (Rendering|Material|SetOverlayMaterial (Variables|Default|GetSM_Plane_Body) 0 :!class /Script/Engine.MeshComponent))

(event Input|EnhancedActionEvents|EnhancedInputActionIA_MoveFowBack
  (params (ActionValue :type Float%20%28double-precision%29) (ElapsedSeconds :type Float%20%28double-precision%29) (TriggeredSeconds :type Float%20%28double-precision%29) (InputAction :type Input%20Action%20Object%20Reference :default "/Game/Inputs/IA_MoveFowBack.IA_MoveFowBack"))
  (bind _arrow (Variables|Default|GetArrow))
  (bind _returnvalue (Math|Vector|GetForwardVector _arrow))
  (bind _returnvalue_2 (* ActionValue _returnvalue))
  ;[0 0.02045 0.15 0.5] Basic movement and spawn player ui
  (Class|PawnMovementComponent|AddInputVector (Variables|Default|GetFloatingPawnMovement) (Math|Vector|MakeVector (.x _returnvalue_2) (.y _returnvalue_2) 0.0) false))

(event Input|EnhancedActionEvents|EnhancedInputActionIA_MoveLeftRight
  (params (ActionValue :type Float%20%28double-precision%29) (ElapsedSeconds :type Float%20%28double-precision%29) (TriggeredSeconds :type Float%20%28double-precision%29) (InputAction :type Input%20Action%20Object%20Reference :default "/Game/Inputs/IA_MoveLeftRight.IA_MoveLeftRight"))
  (bind _arrow (Variables|Default|GetArrow))
  (bind _returnvalue (Math|Vector|GetRightVector _arrow))
  (bind _returnvalue_2 (* ActionValue _returnvalue))
  ;[0 0.02045 0.15 0.5] Basic movement and spawn player ui
  (Class|PawnMovementComponent|AddInputVector (Variables|Default|GetFloatingPawnMovement) (Math|Vector|MakeVector (.x _returnvalue_2) (.y _returnvalue_2) 0.0) false))

(event Input|EnhancedActionEvents|EnhancedInputActionIA_MoveUpDown
  (params (ActionValue :type Float%20%28double-precision%29) (ElapsedSeconds :type Float%20%28double-precision%29) (TriggeredSeconds :type Float%20%28double-precision%29) (InputAction :type Input%20Action%20Object%20Reference :default "/Game/Inputs/IA_MoveUpDown.IA_MoveUpDown"))
  ;[0 0.02045 0.15 0.5] Basic movement and spawn player ui
  (Class|PawnMovementComponent|AddInputVector (Variables|Default|GetFloatingPawnMovement) (Math|Vector|MakeVector 0.0 0.0 ActionValue) false))

(event Input|EnhancedActionEvents|EnhancedInputActionIA_2ndFire
  (params (ActionValue :type Boolean) (ElapsedSeconds :type Float%20%28double-precision%29) (TriggeredSeconds :type Float%20%28double-precision%29) (InputAction :type Input%20Action%20Object%20Reference :default "/Game/Inputs/IA_2ndFire.IA_2ndFire"))
  (bind _arrow (Variables|Default|GetArrow))
  (bind _returnvalue (Transformation|GetWorldTransform _arrow))
  ;[0.15 0 0.1216 0.5] Shooting and Alt Modes
  (Utilities|FlowControl|Delay 0.8)
  (Audio|PlaySound2D "/Game/AudioFile/Sci-Fi_Gun_1-1.Sci-Fi_Gun_1-1" 1.0 1.0 0.0 0 0)
  (switch int (Variables|Default|GetAltFire)
    (:0
      (Game|SpawnActorfromClass "/Game/Blueprints/BP_ProjectileBase_PlayerMissle.BP_ProjectileBase_PlayerMissle_C" (Math|Transform|MakeTransform (.location _returnvalue) (.rotation _returnvalue) "1.000000,1.000000,1.000000") "AdjustIfPossibleButAlwaysSpawn" "MultiplyWithRoot" 0 self :!label _label))
    (:1
      (for _index (range 0 1)
        (Game|SpawnActorfromClass "/Game/Blueprints/BP_ProjectileBase_PlayerMissle.BP_ProjectileBase_PlayerMissle_C" (Math|Transform|MakeTransform (Transformation|GetActorLocation) (Math|Rotator|MakeRotator 0.0 0.0 (+ (* _index 2.7e+02) 45.0 (.yaw (Transformation|GetWorldRotation (Variables|Default|GetArrow))))) "1.000000,1.000000,1.000000") "AdjustIfPossibleButAlwaysSpawn" "MultiplyWithRoot" 0 self)
        (goto _label)))))

(event Input|EnhancedActionEvents|EnhancedInputActionIA_Pause
  (params (ActionValue :type Boolean) (ElapsedSeconds :type Float%20%28double-precision%29) (TriggeredSeconds :type Float%20%28double-precision%29) (InputAction :type Input%20Action%20Object%20Reference :default "/Game/Inputs/IA_Pause.IA_Pause"))
  (bind _returnvalue (Pawn|GetLocalViewingPlayerController))
  ;[0 0.02045 0.15 0.5] Handles Pause Screen
  (:Completed
    (Utilities|FlowControl|FlipFlop
      (:A
        (bind _returnvalue_2 (UserInterface|CreateWidget "/Game/Widgets/WBP_PauseScreen.WBP_PauseScreen_C" (Pawn|GetLocalViewingPlayerController)))
        (UserInterface|Viewport|AddtoViewport _returnvalue_2 0)
        (Game|SetGamePaused true)
        (Input|SetInputModeGameandUI _returnvalue _returnvalue_2 "DoNotLock" false true)
        (Variables|/Script/Engine.PlayerController|SetbShowMouseCursor _returnvalue true))
      (:B
        (Widget|RemovefromParent _returnvalue_2)
        (Game|SetGamePaused false)
        (Input|SetInputModeGameOnly _returnvalue false)
        (Variables|/Script/Engine.PlayerController|SetbShowMouseCursor _returnvalue false)))))

(event Input|EnhancedActionEvents|EnhancedInputActionIA_1stFire
  (params (ActionValue :type Boolean) (ElapsedSeconds :type Float%20%28double-precision%29) (TriggeredSeconds :type Float%20%28double-precision%29) (InputAction :type Input%20Action%20Object%20Reference :default "/Game/Inputs/IA_1stFire.IA_1stFire"))
  (bind _arrow (Variables|Default|GetArrow))
  (bind _arrow_2 (Variables|Default|GetArrow))
  (bind _returnvalue (Transformation|GetWorldTransform _arrow))
  (bind _returnvalue_2 (Transformation|GetWorldTransform _arrow_2))
  ;[0.15 0 0.1216 0.5] Shooting and Alt Modes
  (Utilities|FlowControl|Delay 0.2)
  (Audio|PlaySound2D "/Game/AudioFile/Sci-Fi_Gun_1-1.Sci-Fi_Gun_1-1" 0.7 1.0 0.0 0 0)
  (switch int (Variables|Default|GetAltFire)
    (:0
      (Game|SpawnActorfromClass "/Game/Blueprints/BP_ProjectileBase_PlayerBullet.BP_ProjectileBase_PlayerBullet_C" (Math|Transform|MakeTransform (.location _returnvalue_2) (.rotation _returnvalue_2) "1.000000,1.000000,1.000000") "AdjustIfPossibleButAlwaysSpawn" "MultiplyWithRoot" 0 self))
    (:1
      (bind _isa (Utilities|FlowControl|FlipFlop)
        (:A
          _)
        (:B
          _))
      (Game|SpawnActorfromClass "/Game/Blueprints/BP_ProjectileBase_PlayerBullet.BP_ProjectileBase_PlayerBullet_C" (Math|Transform|MakeTransform (+ (Math|Vector|SelectVector "0.000000,250.000000,0.000000" "0.000000,-250.000000,0.000000" _isa) (.location _returnvalue)) (.rotation _returnvalue) "1.000000,1.000000,1.000000") "AdjustIfPossibleButAlwaysSpawn" "MultiplyWithRoot" 0 self))))

(event EventBeginPlay
  (bind _returnvalue (Class|InputDeviceLibrary|GetPlayerControllerfromInputDevice))
  (Input|SetInputModeGameOnly _returnvalue false))

(event EventPossessed
  (params (NewController :type Controller%20Object%20Reference))
  ;[0 0.02045 0.15 0.5] Basic movement and spawn player ui
  (bind _asplayer_controller (Utilities|Casting|CastToPlayerController NewController))
  (Input|AddMappingContext (PlayerController|LocalPlayerSubsystems|GetEnhancedInputLocalPlayerSubsystem _asplayer_controller) "/Game/Inputs/IMC_SHMUP.IMC_SHMUP" 0 "(bIgnoreAllPressedKeysUntilRelease=True,bForceImmediately=False,bNotifyUserSettings=False)")
  (bind _returnvalue (UserInterface|CreateWidget "/Game/Widgets/WBP_PlayerPawnWidget.WBP_PlayerPawnWidget_C" _asplayer_controller))
  (bind _output_get (Variables|Default|SetWidget _returnvalue))
  (UserInterface|Viewport|AddtoViewport _output_get 0))

(event EventEndPlay
  (params (EndPlayReason :type EEndPlayReason%20Enum :default "Destroyed"))
  ;[0 0.02045 0.15 0.5] Basic movement and spawn player ui
  (Widget|RemovefromParent (Variables|Default|GetWidget))
  (Variables|Default|SetWidget 0)
  (Utilities|Platform|CollectGarbage))

(event Game|Damage|EventAnyDamage
  (params (Damage :type Float%20%28single-precision%29) (DamageType :type Damage%20Type%20Object%20Reference) (InstigatedBy :type Controller%20Object%20Reference) (DamageCauser :type Actor%20Object%20Reference))
  ;[0.15 0.15 0.15 0.5] Updates player Health on damage
  (bind _output_get (Variables|Default|SetHealth (Math|Float|Max(Float) (- (Variables|Default|GetHealth) Damage) 0.0)))
  (Utilities|FlowControl|Sequence
    (:then_0
      (if (== _output_get 0.0)
        (CallFunction|RespawnPlayerpawn)
        (else
          (CallFunction|HitSequence))))
    (:then_1
      (Default|SetHealth (Variables|Default|GetWidget) (Math|Float|SafeDivide (Variables|Default|GetHealth) (Variables|Default|GetMaxHealth))))))

(event EventTick
  (params (DeltaSeconds :type Float%20%28single-precision%29))
  ;[0.15 0 0.1216 0.5] Handles Smoooth movement (interpoling)
  (Utilities|FlowControl|Sequence
    (:then_0
      (Transformation|SetWorldRotation (Variables|Default|GetRotationalOffset) (Math|Rotator|MakeRotator 0.0 0.0 (.yaw (Math|Rotator|FindLookatRotation (Transformation|GetActorLocation) (.Location (Collision|BreakHitResult (.HitResult (Game|Player|GetHitResultUnderCursorbyChannel (Pawn|GetLocalViewingPlayerController) "TraceTypeQuery2" true))))))) false false))
    (:then_1
      (bind _output_get (Variables|Default|SetTargetPitch (* (Input|EnhancedActionValues|GetIA_MoveFowBack) -1.0)))
      (bind _output_get_2 (Variables|Default|SetCurrentPitch (Math|Interpolation|FInterpTo (Variables|Default|GetCurrentPitch) _output_get (Utilities|Time|GetWorldDeltaSeconds) 1.0)))
      (Transformation|SetActorRotation (Math|Rotator|MakeRotator (* (stale _output_get_4) (Variables|Default|GetMaxRoll)) (* _output_get_2 (Variables|Default|GetMaxPitch)) (stale _output_get_6)) :!label _label))
    (:then_2
      (bind _output_get_3 (Variables|Default|SetTargetRoll (Input|EnhancedActionValues|GetIA_MoveLeftRight)))
      (bind _output_get_4 (Variables|Default|SetCurrentRoll (Math|Interpolation|FInterpTo (Variables|Default|GetCurrentRoll) _output_get_3 (Utilities|Time|GetWorldDeltaSeconds) 1.0)))
      (goto _label))
    (:then_3
      (bind _output_get_5 (Variables|Default|SetTargetYAW (.yaw (Transformation|GetWorldRotation (Variables|Default|GetArrow)))))
      (bind _output_get_6 (Variables|Default|SetCurrentYAW (.yaw (Math|Interpolation|RInterpTo (Math|Rotator|MakeRotator 0.0 0.0 (Variables|Default|GetCurrentYAW)) (Math|Rotator|MakeRotator 0.0 0.0 _output_get_5) (Utilities|Time|GetWorldDeltaSeconds) 0.0))))
      (goto _label))))

(event Input|KeyboardEvents|DebugKeyLeftAlt
  (params (Key :type Key%20Structure :default "None") (ActionValue :type Input%20Action%20Value%20Structure))
  ;[0.15 0 0.1216 0.5] Shooting and Alt Modes
  (:Released
    (Variables|Default|SetAltFire (Math|Integer|%(Integer) (+ (Variables|Default|GetAltFire) 1) 2))))

(fn ConstructionScript)