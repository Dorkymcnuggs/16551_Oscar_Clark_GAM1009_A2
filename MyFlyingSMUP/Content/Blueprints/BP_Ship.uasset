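; BP_Ship is a player-controlled ship pawn that moves and fires bullets through Enhanced Input.
; On possession it adds an input mapping context, and two move actions feed world X and Y input into a FloatingPawnMovement component.
; The fire action spawns BP_Ship_Bullet at the Arrow component's location after a short Delay, which also throttles repeated triggers.
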(event `self.ReceivePossessed`
  (params (NewController :type "Controller Object Reference"))
  ; Adds mapped key binds on possess
  (bind _asplayer_controller (cast `PlayerController` NewController))
  (`EnhancedInputSubsystemInterface.AddMappingContext` (pcsubsystem `EnhancedInputLocalPlayerSubsystem` _asplayer_controller) null 0 (struct)))

(event `EnhancedInput|/Game/Inputs/IA_MoveFowBack`
  (params (ActionValue :type "Float (double-precision)") (ElapsedSeconds :type "Float (double-precision)") (TriggeredSeconds :type "Float (double-precision)") (InputAction :type "InputAction Object Reference" :default "/Game/Inputs/IA_MoveFowBack.IA_MoveFowBack"))
  ; Setup movement for plane
  (:`Triggered`
    (`PawnMovementComponent.AddInputVector` (`self.FloatingPawnMovement`) (`KismetMathLibrary.MakeVector` ActionValue) false)))

(event `EnhancedInput|/Game/Inputs/IA_MoveLeftRight`
  (params (ActionValue :type "Float (double-precision)") (ElapsedSeconds :type "Float (double-precision)") (TriggeredSeconds :type "Float (double-precision)") (InputAction :type "InputAction Object Reference" :default "/Game/Inputs/IA_MoveLeftRight.IA_MoveLeftRight"))
  ; Setup movement for plane
  (:`Triggered`
    (`PawnMovementComponent.AddInputVector` (`self.FloatingPawnMovement`) (`KismetMathLibrary.MakeVector` 0.0 ActionValue) false)))

(event `EnhancedInput|/Game/Inputs/IA_1stFire`
  (params (ActionValue :type Boolean) (ElapsedSeconds :type "Float (double-precision)") (TriggeredSeconds :type "Float (double-precision)") (InputAction :type "InputAction Object Reference" :default "/Game/Inputs/IA_1stFire.IA_1stFire"))
  (:`Triggered`
    (`KismetSystemLibrary.Delay` 0.2)
    (`|SpawnActorFromClass` "/Game/Blueprints/Projectiles/BP_Ship_Bullet.BP_Ship_Bullet_C" (`KismetMathLibrary.MakeTransform` (`SceneComponent.K2_GetComponentLocation` (`self.Arrow`))) "Undefined" "MultiplyWithRoot" null null)))

(fn `UserConstructionScript`)