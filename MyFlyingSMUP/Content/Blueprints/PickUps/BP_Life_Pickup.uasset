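; Life pickup actor that can home in on a collector and sends a stat pickup message to whatever overlaps it.
; BeginPlay presets the player pawn as homing target, and CollectPickUp retargets the projectile movement and enables strong homing.
; Sphere overlap sends the message, then plays a sound, disables collision, hides and destroys the actor after a brief delay.
; GetHealthValue returns zero here.
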(event `self.ReceiveBeginPlay`
  (set `ProjectileMovementComponent.HomingTargetComponent` (`Actor.RootComponent` (`GameplayStatics.GetPlayerPawn` 0)) (`self.ProjectileMovement`)))

(event `self.Sphere.OnComponentBeginOverlap`
  (params (OverlappedComponent :type "PrimitiveComponent Object Reference") (OtherActor :type "Actor Object Reference") (OtherComp :type "PrimitiveComponent Object Reference") (OtherBodyIndex :type Integer) (bFromSweep :type Boolean) (SweepResult :type "HitResult Structure (by ref)"))
  (message `/Game/GameFrame/BPI_SCHMUP.ApplyStatPickUp` OtherActor)
  (`self.DestroySelf`))

(event `self.CollectPickUp`
  (params (HomingTarget :type "/Game/Blueprints/BP_Player Object Reference"))
  (bind _projectilemovement (`self.ProjectileMovement`))
  (set `ProjectileMovementComponent.HomingTargetComponent` (`Actor.RootComponent` HomingTarget) _projectilemovement)
  (set `ProjectileMovementComponent.bIsHomingProjectile` true _projectilemovement)
  (set `ProjectileMovementComponent.HomingAccelerationMagnitude` 40000.0 _projectilemovement))

(event `DestroySelf`
  (`GameplayStatics.PlaySound2D` "/Game/AudioFile/SW_Pickup.SW_Pickup" 1.0 1.0 0.0 null null)
  (`PrimitiveComponent.SetCollisionEnabled` (`self.Sphere`) "NoCollision")
  (`self.SetActorHiddenInGame` self true)
  (`KismetSystemLibrary.Delay` 0.1)
  (`self.K2_DestroyActor` self))

(fn `ApplyStatPickUp`
  (returns (Stats :type "/Game/Blueprints/PickUps/S_Pickup Structure"))
  (return (`self.S_Pickup`)))

(fn `GetHealthValue`
  (returns (HealthValue :type "Float (double-precision)"))
  (return 0.0))

(fn `UserConstructionScript`)