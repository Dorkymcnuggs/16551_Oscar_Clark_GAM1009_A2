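; BP_Enemy is an enemy actor with UFO and static meshes that takes damage and explodes when its health runs out.
; AnyDamage lowers clamped health, sends the health ratio to its widget component and spawns a BP_Damage_PopUp carrying the damage amount.
; Surviving hits play a sound and briefly flash a damage overlay material on both meshes.
; At zero health it plays a sound, spawns BP_Explosion and destroys itself.
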(event `self.ReceiveAnyDamage`
  (params (Damage :type "Float (single-precision)") (DamageType :type "DamageType Object Reference") (InstigatedBy :type "Controller Object Reference") (DamageCauser :type "Actor Object Reference"))
  ;[0 0.15 0.0326 0.5] Setting enemy health when hit
  (set `self.Health` (`KismetMathLibrary.FMax` (- (`self.Health`) Damage)))
  (`|ExecutionSequence`
    (:`then_0`
      ;[0.15 0 0 0.5] Set Health UI widget to current health
      (message `/Game/GameFrame/BPI_SCHMUP.SetHealth` (`WidgetComponent.GetUserWidgetObject` (`self.Widget`)) (`KismetMathLibrary.SafeDivide` (`self.Health`) (`self.MaxHealth`))))
    (:`then_1`
      ;[0.15 0.006155 0 0.5] Set Damage Widget Location
      (`|SpawnActorFromClass` "/Game/Widgets/BP_Damage_PopUp.BP_Damage_PopUp_C" (`KismetMathLibrary.MakeTransform` (`self.K2_GetActorLocation`)) "Undefined" "MultiplyWithRoot" null Damage null))
    (:`then_3`
      ;[0.15 0 0 0.5] Determines if enemy is dead
      (if (== (`self.Health`) 0.0)
        (`self.KillSequence`)
        (else
          (`self.HitSequence`))))))

(event `HitSequence`
  ;[0.05301 0.129 0.15 0.5] On hit event displays flashing colour
  (`GameplayStatics.PlaySound2D` "/Game/AudioFile/MS_Hit.MS_Hit" 1.0 1.0 0.0 null null)
  (`MeshComponent.SetOverlayMaterial` (`self.StaticMesh`) "/Game/Materials/M_OverlayDamage.M_OverlayDamage")
  (`MeshComponent.SetOverlayMaterial` (`self.UFO`) "/Game/Materials/M_OverlayDamage.M_OverlayDamage")
  (`KismetSystemLibrary.Delay` 2.0)
  (`MeshComponent.SetOverlayMaterial` (`self.StaticMesh`) null)
  (`MeshComponent.SetOverlayMaterial` (`self.UFO`) null))

(event `KillSequence`
  ;[0.05301 0.129 0.15 0.5] On Kill event destroys actor and play explosion effect
  (`GameplayStatics.PlaySound2D` "/Game/AudioFile/MS_Exploxion.MS_Exploxion" 1.0 1.0 0.0 null null)
  (`|SpawnActorFromClass` "/Game/Blueprints/BP_Explosion.BP_Explosion_C" (`self.GetTransform`) "Undefined" "MultiplyWithRoot" null null)
  (`self.K2_DestroyActor`))

(fn `UserConstructionScript`)