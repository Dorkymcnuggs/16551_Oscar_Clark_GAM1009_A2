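; BP_ForceField is a force field actor that damages whatever overlaps it and wears out after a limited number of contacts.
; Each overlap applies fixed damage to the other actor and decrements HitCap, destroying the field at zero.
; Damage received by the field leaves HitCap untouched, playing a hit sound and briefly showing a shield-damage overlay material on Sphere1 before clearing it.
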(event `self.ReceiveActorBeginOverlap`
  (params (OtherActor :type "Actor Object Reference"))
  (`GameplayStatics.ApplyDamage` OtherActor 100.0)
  (bind _result (`/Engine/EditorBlueprintResources/StandardMacros.DecrementInt` (`self.HitCap`))
    (:`  `
      (if (== _result 0)
        (`self.K2_DestroyActor`)))))

(event `self.ReceiveAnyDamage`
  (params (Damage :type "Float (single-precision)") (DamageType :type "DamageType Object Reference") (InstigatedBy :type "Controller Object Reference") (DamageCauser :type "Actor Object Reference"))
  (`GameplayStatics.PlaySound2D` "/Game/AudioFile/MS_Hit.MS_Hit" 1.0 1.0 0.0 null null)
  (`MeshComponent.SetOverlayMaterial` (`self.Sphere1`) "/Game/Materials/M_OverlayShieldDamage.M_OverlayShieldDamage")
  (`KismetSystemLibrary.Delay` 2.0)
  (`MeshComponent.SetOverlayMaterial` (`self.Sphere1`) null))

(fn `UserConstructionScript`)