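; Boss enemy that flies into frame, then strafes side to side while firing spread shots.
; After a delay on BeginPlay it activates the MoveSideways component and starts a looping ShootBullet timer.
; Each volley spawns three enemy bullets from each of two cannon points (Arrow and Cannon2): one straight and two yawed 45 degrees either side, all oriented from the Arrow's rotation.
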(event `self.ReceiveBeginPlay`
  ;[0.000825 0.01081 0.15 0.5] This changes movement to allow a fly into frame and then side to side
  (`KismetSystemLibrary.Delay` 6.0)
  (`ActorComponent.Activate` (`self.MoveSideways`) false)
  (`KismetSystemLibrary.K2_SetTimerDelegate` (delegate `ShootBullet`) 2.0 true))

(event `ShootBullet`
  (bind (_returnvalue_roll _returnvalue_pitch _returnvalue_yaw) (`KismetMathLibrary.BreakRotator` (`SceneComponent.K2_GetComponentRotation` (`self.Arrow`))))
  (bind (_returnvalue_roll_2 _returnvalue_pitch_2 _returnvalue_yaw_2) (`KismetMathLibrary.BreakRotator` (`SceneComponent.K2_GetComponentRotation` (`self.Arrow`))))
  ;[0.000825 0.01081 0.15 0.5] Sets location to fire from
  (set `self.BossCanon1` (`SceneComponent.K2_GetComponentLocation` (`self.Arrow`)))
  (set `self.BossCanon2` (`SceneComponent.K2_GetComponentLocation` (`self.Cannon2`)))
  (`|ExecutionSequence`
    (:`then_0`
      ;[0.09699 0.01124 0.15 0.5] Causes bos to shoot a shotgun of three bullets at designated points
      (for _index (range 2)
        (`|SpawnActorFromClass` "/Game/Blueprints/Projectiles/BP_ProjectileBase_EnemyBullet.BP_ProjectileBase_EnemyBullet_C" (`KismetMathLibrary.MakeTransform` (`self.BossCanon2`) (`KismetMathLibrary.MakeRotator` 0.0 0.0 (+ (* _index 270.0) 45.0 _returnvalue_yaw_2))) "AdjustIfPossibleButAlwaysSpawn" "MultiplyWithRoot" null self)))
    (:`then_1`
      (`|SpawnActorFromClass` "/Game/Blueprints/Projectiles/BP_ProjectileBase_EnemyBullet.BP_ProjectileBase_EnemyBullet_C" (`KismetMathLibrary.MakeTransform` (`self.BossCanon2`) (`SceneComponent.K2_GetComponentRotation` (`self.Arrow`))) "AdjustIfPossibleButAlwaysSpawn" "MultiplyWithRoot" null self))
    (:`then_2`
      (for _index_2 (range 2)
        (`|SpawnActorFromClass` "/Game/Blueprints/Projectiles/BP_ProjectileBase_EnemyBullet.BP_ProjectileBase_EnemyBullet_C" (`KismetMathLibrary.MakeTransform` (`self.BossCanon1`) (`KismetMathLibrary.MakeRotator` 0.0 0.0 (+ (* _index_2 270.0) 45.0 _returnvalue_yaw))) "AdjustIfPossibleButAlwaysSpawn" "MultiplyWithRoot" null self)))
    (:`then_3`
      (`|SpawnActorFromClass` "/Game/Blueprints/Projectiles/BP_ProjectileBase_EnemyBullet.BP_ProjectileBase_EnemyBullet_C" (`KismetMathLibrary.MakeTransform` (`self.BossCanon1`) (`SceneComponent.K2_GetComponentRotation` (`self.Arrow`))) "AdjustIfPossibleButAlwaysSpawn" "MultiplyWithRoot" null self))))

(fn `UserConstructionScript`
  (`parent.UserConstructionScript`))