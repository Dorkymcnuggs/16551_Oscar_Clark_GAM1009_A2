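; Enemy wave spawner actor that runs the waves from WaveData in order, starting at BeginPlay.
; Each wave waits its initial delay, then spawns every listed enemy class on each timed step until the spawn count is reached.
; Regular enemies appear at random points between the left and right limit components, bosses at the root.
; It polls until EnemiesRemain, which this graph never decrements, hits zero before advancing.
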(event `self.ReceiveBeginPlay`
  (set `self.LastWaveIndex` (`KismetArrayLibrary.Array_LastIndex` (`/Game/EnemyWaveSyst/PDA_Level.Waves` (`self.WaveData`))))
  (`self.BeginSetOfWaves`))

(event `BeginSetOfWaves`
  ;[0.000825 0.01081 0.15 0.5] Sets first wave
  (set `self.CurWaveIndex` 0)
  (`self.NextWave`))

(event `NextWave`
  ;[0.000825 0.01081 0.15 0.5] Checks wave
  (if (not (> (`self.CurWaveIndex`) (`self.LastWaveIndex`)))
    (`KismetSystemLibrary.Delay` (`.InitialDelay_10_D63332254280005B89A4FE83CF495E42` (break `/Game/EnemyWaveSyst/S_Wave` (`|GetArrayItem` (`/Game/EnemyWaveSyst/PDA_Level.Waves` (`self.WaveData`)) (`self.CurWaveIndex`)))))
    (`self.BeginSpawn`)))

(event `BeginSpawn`
  (bind ((`SpawnInterval_13_D4B400D842FEFE3C8C70299CE38E5B19` _spawninterval) (`SpawnCount_16_BC9150B44205CC9F724CB483E10A96EA` _spawncount) (`Enemies_19_FFB8D6B7439A211E10A9C1B64A3676FE` _enemies)) (break `/Game/EnemyWaveSyst/S_Wave` (`|GetArrayItem` (`/Game/EnemyWaveSyst/PDA_Level.Waves` (`self.WaveData`)) (`self.CurWaveIndex`))))
  ;[0.000825 0.01081 0.15 0.5] Checks requirements for spawns
  (set `self.CurrentSpawn` 0)
  (set `self.Spawn Interval` _spawninterval)
  (bind _output_get (set `self.NumToSpawn` _spawncount))
  (set `self.Enemies` _enemies)
  (set `self.EnemiesRemain` _output_get)
  (`self.NextSpawn`))

(event `NextSpawn`
  (bind _enemies_enemy (break `/Game/EnemyWaveSyst/S_Enemies` (`self.Enemies`)))
  ;[0.000825 0.01081 0.15 0.5] Spawns number of enemies
  (if (== (`self.CurrentSpawn`) (`self.NumToSpawn`))
    (if (== (`self.EnemiesRemain`) 0) :!label _label
      (`/Engine/EditorBlueprintResources/StandardMacros.IncrementInt` (`self.CurWaveIndex`)
        (:`  `
          (`self.NextWave`)))
      (else
        (`KismetSystemLibrary.Delay` 0.2)
        (goto _label)))
    (else
      (for _array_element _enemies_enemy
        (if (`.IsBoss_22_99EB05734AB807CC38E6139D604496FA` (break `/Game/EnemyWaveSyst/S_Wave` (`|GetArrayItem` (`/Game/EnemyWaveSyst/PDA_Level.Waves` (`self.WaveData`)) (`self.CurWaveIndex`))))
          (`|SpawnActorFromClass` _array_element (`KismetMathLibrary.MakeTransform` (`SceneComponent.K2_GetComponentLocation` (`self.DefaultSceneRoot`)) (`self.Rotation`)) "Undefined" "MultiplyWithRoot" null null)
          (else
            (bind _output_get (set `self.Transform` (`KismetMathLibrary.VLerp` (`SceneComponent.K2_GetComponentLocation` (`self.LeftSpawnLim`)) (`SceneComponent.K2_GetComponentLocation` (`self.RightSpawnLim`)) (`KismetMathLibrary.RandomFloat`))))
            (bind _output_get_2 (set `self.Rotation` (`SceneComponent.K2_GetComponentRotation` (`self.LeftSpawnLim`))))
            (`|SpawnActorFromClass` _array_element (`KismetMathLibrary.MakeTransform` _output_get _output_get_2) "Undefined" "MultiplyWithRoot" null null))))
      (`/Engine/EditorBlueprintResources/StandardMacros.IncrementInt` (`self.CurrentSpawn`)
        (:`  `
          (`KismetSystemLibrary.Delay` (`self.Spawn Interval`))
          (`self.NextSpawn`))))))

(fn `UserConstructionScript`)